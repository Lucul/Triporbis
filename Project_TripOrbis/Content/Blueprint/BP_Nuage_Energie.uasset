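; BP_Nuage_Energie is an energy cloud that starts and ends the fuel-pump minigame as the player passes through it.
; On BeginPlay, a timeline moves the actor by driving its X location.
; Box overlaps with the 2DSideScrollerCharacter find BP_Minijeu_PompeEssence actors and call DebutMJessence on entry, Fin on exit.
; DebutMJNuage is empty and the NuageSpawn logic is unconnected.
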(event `self.ReceiveTick`
  (params (DeltaSeconds :type "Float (single-precision)")))

(event `DebutMJNuage`)

(event `self.ReceiveBeginPlay`
  (bind (_direction _location) (`Timeline|Timeline_0` :!via `PlayFromStart`)
    (:`Update`
      (`self.K2_SetActorLocation` (`KismetMathLibrary.MakeVector` _location)))))

(event `self.Box.OnComponentBeginOverlap`
  (params (OverlappedComponent :type "PrimitiveComponent Object Reference") (OtherActor :type "Actor Object Reference") (OtherComp :type "PrimitiveComponent Object Reference") (OtherBodyIndex :type Integer) (bFromSweep :type Boolean) (SweepResult :type "HitResult Structure (by ref)"))
  (cast `/Game/2DSideScrollerBP/Blueprints/2DSideScrollerCharacter` OtherActor)
  (bind _outactors (`GameplayStatics.GetAllActorsOfClass` "/Game/Blueprint/BP_Minijeu_PompeEssence.BP_Minijeu_PompeEssence_C"))
  (`/Game/Blueprint/BP_Minijeu_PompeEssence.DebutMJessence` _outactors))

(event `self.Box.OnComponentEndOverlap`
  (params (OverlappedComponent :type "PrimitiveComponent Object Reference") (OtherActor :type "Actor Object Reference") (OtherComp :type "PrimitiveComponent Object Reference") (OtherBodyIndex :type Integer))
  (cast `/Game/2DSideScrollerBP/Blueprints/2DSideScrollerCharacter` OtherActor)
  (bind _outactors (`GameplayStatics.GetAllActorsOfClass` "/Game/Blueprint/BP_Minijeu_PompeEssence.BP_Minijeu_PompeEssence_C"))
  (`/Game/Blueprint/BP_Minijeu_PompeEssence.Fin` _outactors))

(fn `UserConstructionScript`)