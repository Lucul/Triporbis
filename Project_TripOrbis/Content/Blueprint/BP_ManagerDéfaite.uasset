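; Defeat manager that watches the player's fuel (Essence), supplies (Vivres) and ship health (VieVaisseau) for a loss.
; BeginPlay caches player 0's character as a 2DSideScrollerCharacter, then Tick polls each resource through its own custom event.
; When a resource reaches zero or below, that check's separate DoOnce prints "DEFAITE", with no further game-over logic.
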(event `self.ReceiveBeginPlay`
  (bind _as2dside_scroller_character (cast `/Game/2DSideScrollerBP/Blueprints/2DSideScrollerCharacter` (`GameplayStatics.GetPlayerCharacter` 0)))
  (set `self.RefPlayer` _as2dside_scroller_character))

(event `self.ReceiveTick`
  (params (DeltaSeconds :type "Float (single-precision)"))
  (`self.Comp Essence`)
  (`self.Comp Vie Vaisseau`)
  (`self.Comp Vivres`))

(event `Comp Essence`
  (if (<= (`/Game/2DSideScrollerBP/Blueprints/2DSideScrollerCharacter.Essence` (`self.RefPlayer`)) 0.0)
    (`/Engine/EditorBlueprintResources/StandardMacros.DoOnce` false
      (:`Completed`
        (`KismetSystemLibrary.PrintString` "DEFAITE")))))

(event `Comp Vivres`
  (if (<= (`/Game/2DSideScrollerBP/Blueprints/2DSideScrollerCharacter.Vivres` (`self.RefPlayer`)) 0.0)
    (`/Engine/EditorBlueprintResources/StandardMacros.DoOnce` false
      (:`Completed`
        (`KismetSystemLibrary.PrintString` "DEFAITE")))))

(event `Comp Vie Vaisseau`
  (if (<= (`/Game/2DSideScrollerBP/Blueprints/2DSideScrollerCharacter.VieVaisseau` (`self.RefPlayer`)) 0.0)
    (`/Engine/EditorBlueprintResources/StandardMacros.DoOnce` false
      (:`Completed`
        (`KismetSystemLibrary.PrintString` "DEFAITE")))))

(fn `UserConstructionScript`)