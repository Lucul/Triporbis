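; Click-to-repair minigame that has the player click a random number of times to restore ship health.
; Starting it flags the minigame on the player, rolls the click target and launches a one-second Delay countdown loop, which triggers nothing at zero.
; Each OnClick decrements the target; reaching zero sets ship health to a fixed value, notifies the HUD, clears the flag and marks the win.
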(event `DébutMJClicRéparation`
  ;[1 1 1] Début
  (set `/Game/2DSideScrollerBP/Blueprints/2DSideScrollerCharacter.Mini jeu en cours` true (`self.Ref player`))
  (set `self.nombre de fois a toucher` (`KismetMathLibrary.RandomIntegerInRange` 15 25))
  (`self.Commencement du timer`))

(event `self.ReceiveBeginPlay`
  ;[1 1 1] Event beginplay et ref player
  (bind _as2dside_scroller_character (cast `/Game/2DSideScrollerBP/Blueprints/2DSideScrollerCharacter` (`GameplayStatics.GetPlayerCharacter` 0)))
  (set `self.Ref player` _as2dside_scroller_character))

(event `Commencement du timer`
  ;[1 1 1] Timer
  (if (not (`self.Gagné?`))
    (`KismetSystemLibrary.Delay` 1.0 :!label _label)
    (if (not (<= (`self.Minuterie condiction de defaite`) 0))
      (`/Engine/EditorBlueprintResources/StandardMacros.DecrementInt` (`self.Minuterie condiction de defaite`)
        (:`  `
          (goto _label))))))

(event `On Click`
  (bind _nombre_de_fois_a_toucher (`self.nombre de fois a toucher`))
  ;[1 1 1] On Clic
  (`KismetSystemLibrary.PrintString` (`KismetStringLibrary.Conv_IntToString` _nombre_de_fois_a_toucher))
  (bind _result (`/Engine/EditorBlueprintResources/StandardMacros.DecrementInt` _nombre_de_fois_a_toucher)
    (:`  `
      (if (<= _result 0)
        (set `/Game/2DSideScrollerBP/Blueprints/2DSideScrollerCharacter.VieVaisseau` 0.3 (`self.Ref player`))
        (bind _foundwidgets (`WidgetBlueprintLibrary.GetAllWidgetsOfClass` "/Game/2DSideScrollerBP/UI/WGT_HUD.WGT_HUD_C"))
        (`/Game/2DSideScrollerBP/UI/WGT_HUD.FinMiniJeuClick` _foundwidgets)
        (set `/Game/2DSideScrollerBP/Blueprints/2DSideScrollerCharacter.Mini jeu en cours` false (`self.Ref player`))
        (set `self.Gagné?` true)))))

(fn `UserConstructionScript`)