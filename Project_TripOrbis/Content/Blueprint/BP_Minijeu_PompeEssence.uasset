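; Fuel pump minigame in which the player alternates up and down arrow inputs to refill their Essence.
; Start and end events toggle the input gate and the MiniJeuEnCours flag on the 2DSideScrollerCharacter.
; A boolean enforces alternation between the two arrow events, which feed a shared FlipFlop.
; Only every second valid press, completing one pump stroke, adds a fixed amount of fuel to the player.
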(event `self.ReceiveBeginPlay`
  ;[1 1 1] event begin play et ref player
  (bind _as2dside_scroller_character (cast `/Game/2DSideScrollerBP/Blueprints/2DSideScrollerCharacter` (`GameplayStatics.GetPlayerCharacter` 0)))
  (set `self.Ref player` _as2dside_scroller_character))

(event `DebutMJessence`
  ;[1 1 1] Début MJ
  (set `self.DansNuageNRJ` true)
  (bind _outactors (`GameplayStatics.GetAllActorsOfClass` "/Game/2DSideScrollerBP/Blueprints/2DSideScrollerCharacter.2DSideScrollerCharacter_C"))
  (set `/Game/2DSideScrollerBP/Blueprints/2DSideScrollerCharacter.Mini jeu en cours` true (`|GetArrayItem` _outactors)))

(event `Fin`
  ;[1 1 1] Fin MJ
  (set `self.DansNuageNRJ` false)
  (bind _outactors (`GameplayStatics.GetAllActorsOfClass` "/Game/2DSideScrollerBP/Blueprints/2DSideScrollerCharacter.2DSideScrollerCharacter_C"))
  (set `/Game/2DSideScrollerBP/Blueprints/2DSideScrollerCharacter.Mini jeu en cours` false (`|GetArrayItem` _outactors)))

(event `Flèche du haut event pompe a essance`
  (bind _ref_player (`self.Ref player`))
  ;[1 1 1] input flèche Haut/Bas
  (if (`self.DansNuageNRJ`)
    (if (`self.Haut = true`)
      (set `self.Haut = true` false)
      (`/Engine/EditorBlueprintResources/StandardMacros.FlipFlop` :!label _label
        (:`B`
          (set `/Game/2DSideScrollerBP/Blueprints/2DSideScrollerCharacter.Essence` (+ (`/Game/2DSideScrollerBP/Blueprints/2DSideScrollerCharacter.Essence` _ref_player) 0.8) _ref_player))))))

(event `Flèche du bas event pompe a essence`
  ;[1 1 1] input flèche Haut/Bas
  (if (`self.DansNuageNRJ`)
    (if (not (`self.Haut = true`))
      (set `self.Haut = true` true)
      (goto _label))))

(fn `UserConstructionScript`)