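; Manager that spawns BP_Etoile actors at the Spawn component's X/Y and a random height, capped by a maximum on-map count.
; Spawnetoile makes the initial staggered batch, repeating after random delays while the player character is airborne, up to a fixed count.
; When a star overlaps the Gauche component, the live count drops, a replacement spawn is requested, and DestroyActor is called.
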(event `self.ReceiveBeginPlay`
  (bind _as2dside_scroller_character (cast `/Game/2DSideScrollerBP/Blueprints/2DSideScrollerCharacter` (`GameplayStatics.GetPlayerCharacter` 0)))
  (set `self.Ref player` _as2dside_scroller_character))

(event `Spawn etoile`
  (`self.Nuage_spawn` :!label _label)
  (if (`/Game/2DSideScrollerBP/Blueprints/2DSideScrollerCharacter.joueur en l'air` (`self.Ref player`))
    (bind _output_get (set `self.Nombre_Nuage_Départ` (+ (`self.Nombre_Nuage_Départ`) 1)))
    (if (not (>= _output_get 5))
      (`KismetSystemLibrary.Delay` (`KismetMathLibrary.RandomFloatInRange` 0.5 1.5))
      (goto _label))))

(event `self.Gauche.OnComponentBeginOverlap`
  (params (OverlappedComponent :type "PrimitiveComponent Object Reference") (OtherActor :type "Actor Object Reference") (OtherComp :type "PrimitiveComponent Object Reference") (OtherBodyIndex :type Integer) (bFromSweep :type Boolean) (SweepResult :type "HitResult Structure (by ref)"))
  (cast `/Game/Blueprint/BP_Etoile` OtherActor)
  (set `self.Nuage_on_map` (- (`self.Nuage_on_map`) 1))
  (`self.Nuage_spawn`)
  (`self.K2_DestroyActor`))

(event `Nuage_spawn`
  (bind (_returnvalue_x _returnvalue_y) (`KismetMathLibrary.BreakVector` (`SceneComponent.K2_GetComponentLocation` (`self.spawn`))))
  (`/Engine/EditorBlueprintResources/StandardMacros.CompareInt` (`self.Nuage_on_map`) (`self.Nuage_max_on_map`)
    (:`<`
      (`|SpawnActorFromClass` "/Game/Blueprint/BP_Etoile.BP_Etoile_C" (`KismetMathLibrary.MakeTransform` (`KismetMathLibrary.MakeVector` _returnvalue_x _returnvalue_y (`KismetMathLibrary.Conv_IntToDouble` (`KismetMathLibrary.RandomIntegerInRange` 270 480)))) "Undefined" "OverrideRootScale" null null)
      (set `self.Nuage_on_map` (+ (`self.Nuage_on_map`) 1)))))

(fn `UserConstructionScript`)